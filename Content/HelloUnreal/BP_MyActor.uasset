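; BP_MyActor is a learning-exercise actor whose StaticMesh shuttles back and forth along X.
; Every Tick calls NewFunction, which, while IsPlay is true, steps X위치 and flips IsMoveRight at each bound to reverse direction.
; Debug prints mark BeginPlay, each Tick and a looping timer that fires OnUpdaterTimer.
; Stepped-move and name-print chains are left unconnected, along with unused operator nodes, and the overlap event is empty.
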(event `self.StaticMesh.OnComponentBeginOverlap`
  (params (OverlappedComponent :type "PrimitiveComponent Object Reference") (OtherActor :type "Actor Object Reference") (OtherComp :type "PrimitiveComponent Object Reference") (OtherBodyIndex :type Integer) (bFromSweep :type Boolean) (SweepResult :type "HitResult Structure (by ref)")))

(event `self.ReceiveBeginPlay`
  (`KismetSystemLibrary.PrintString` "Begin Play")
  (`KismetSystemLibrary.K2_SetTimer` null "OnUpdaterTimer" 0.1 true))

(event `self.ReceiveTick`
  (params (DeltaSeconds :type "Float (single-precision)"))
  (`KismetSystemLibrary.PrintString` "Tick")
  (`self.NewFunction`))

(fn `NewFunction`
  ;[1 1 1] 스위치 생성
  (if (`self.IsPlay`)
    ;[1 1 1] 움직임 조건 제안
    (if (`self.IsMoveRight`)
      ;[1 1 1] X 방향으로 한번 움직인다
      (bind _output_get (set `self.X위치` (+ (`self.X위치`) 1.0)))
      (`SceneComponent.K2_SetRelativeLocation` (`self.StaticMesh`) (`KismetMathLibrary.MakeVector` _output_get) false false)
      (if (> (`self.X위치`) 100.0)
        (set `self.IsMoveRight` false))
      (else
        ;[1 1 1] X 반대 방향으로 한번 움직인다
        (bind _output_get_2 (set `self.X위치` (+ (`self.X위치`) -1.0)))
        (`SceneComponent.K2_SetRelativeLocation` (`self.StaticMesh`) (`KismetMathLibrary.MakeVector` _output_get_2) false false)
        (if (< (`self.X위치`) 0.0)
          (set `self.IsMoveRight` true))))))

(fn `OnUpdaterTimer`
  (`KismetSystemLibrary.PrintString` "timer"))

(fn `UserConstructionScript`)